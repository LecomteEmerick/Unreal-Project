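; Behavior tree decorator that looks for nearby interest points for a creature AI.
; Its condition check sphere-traces around the owner for interest-point object types, ignoring all actors of the owner's class, and takes the first hit cast to InterstPoint.
; On a find it changes the AiState blackboard key and writes the InterestPoint key.
; The check returns false even on success, so it works through these blackboard side effects.
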(fn PerformConditionCheck
  (params (OwnerActor :type Actor%20Object%20Reference))
  (bind _returnvalue (Transformation|GetActorLocation OwnerActor))
  (bind _outactors (Actor|GetAllActorsOfClass (Utilities|GetClass OwnerActor)))
  (bind (_outhits _returnvalue_2) (Collision|MultiSphereTraceForObjects _returnvalue (+ _returnvalue "0, 0,15.000000") 3e+02 (Variables|Default|GetInterestPointType) false _outactors "None"))
  (if _returnvalue_2
    (bind _array_element (Utilities|Array|ForEachLoopwithBreak _outhits :!label _label)
      (:LoopBody
        (bind _asinterst_point (Utilities|Casting|CastToInterstPoint (.HitActor (Collision|BreakHitResult _array_element))))
        (bind _output_get (LocalVariables|SetInterestPointFound _asinterst_point))
        (goto _label Break))
      (:Completed
        (if (!= _output_get 0)
          (Class|BTFunctionLibrary|SetBlackboardValueasEnum (Variables|Default|GetAiState) (Utilities|Enum|LiteralenumAiState "NewEnumerator2"))
          (Class|BTFunctionLibrary|SetBlackboardValueasObject (Variables|Default|GetInterestPoint))
          (return false)
          (else
            (return false)))))
    (else
      (return false))))