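; Behavior tree service for the follower AI that destroys any Creature_Character its line trace hits.
; Each tick it casts the owner to Follower_AI_CON and traces for Pawn objects from the controlled pawn's location, drawing persistent debug lines.
; The trace end is the forward vector times a small scalar without the location added, so it points near the world origin rather than ahead of the pawn.
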(event `self.ReceiveTick`
  (params (OwnerActor :type "Actor Object Reference") (DeltaSeconds :type "Float (single-precision)"))
  (bind _asfollower_ai_con (cast `/Game/Blueprints/AIFolder/Follower_AI_CON` OwnerActor)
    (:`then`
      (bind _returnvalue (`Controller.K2_GetPawn` _asfollower_ai_con))
      (bind _outhit (`KismetSystemLibrary.LineTraceSingleForObjects` :`Start` (`Actor.K2_GetActorLocation` _returnvalue) :`End` (* (`Actor.GetActorForwardVector` _returnvalue) 5.0) :`ObjectTypes` (`|MakeArray` "ObjectTypeQuery3" :!type "EObjectTypeQuery Enum") :`DrawDebugType` "Persistent"))
      (bind _ascreature_character (cast `/Game/Blueprints/Creature_AI_Folder/Creature_Character` (`.HitActor` (`GameplayStatics.BreakHitResult` _outhit))))
      (`Actor.K2_DestroyActor` _ascreature_character))
    (:`CastFailed`
      (`KismetSystemLibrary.PrintString` "Cast failed"))))