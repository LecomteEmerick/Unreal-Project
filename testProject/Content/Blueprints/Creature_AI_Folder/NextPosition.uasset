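; NextPosition is a behavior tree node that picks random wander targets for the creature AI.
; Each tick, it finds the Floor_Blueprint under the controlled Creature_Character and writes a random point to the TargetLocation blackboard key if valid.
; X and Y come from the floor mesh's local bounds, without transforming to world space, and Z from the floor hit.
; Failed casts yield a zero vector.
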(event EventTick
  (params (OwnerActor :type Actor%20Object%20Reference) (DeltaSeconds :type Float%20%28single-precision%29))
  (bind _randomvector (CallFunction|GenerateRandomPosition OwnerActor))
  (if (AI|IsValidAILocation _randomvector)
    (AI|BehaviorTree|SetBlackboardValueasVector (Variables|Default|GetTargetLocation) _randomvector)))

(fn GenerateRandomPosition
  (params (MyActor :type Actor%20Object%20Reference))
  (bind _returnvalue (AI|GetAIController MyActor))
  (bind _ascreature_ai_con (Utilities|Casting|CastToCreature_AI_CON _returnvalue)
    (:then
      (bind _ascreature_character (Utilities|Casting|CastToCreature_Character (Pawn|GetControlledPawn _ascreature_ai_con))
        (:then
          (LocalVariables|SetSaveZ (.Z (Math|Vector|BreakVector (.Location (Collision|BreakHitResult (.HitResult (Utilities|Struct|BreakFindFloorResult (Variables|/Script/Engine.CharacterMovementComponent|GetCurrentFloor (Variables|/Script/Engine.Character|GetCharacterMovement _ascreature_character)))))))))
          (bind _asfloor_blueprint (Utilities|Casting|CastToFloor_Blueprint (.HitActor (Collision|BreakHitResult (.HitResult (Utilities|Struct|BreakFindFloorResult (Variables|/Script/Engine.CharacterMovementComponent|GetCurrentFloor (Variables|/Script/Engine.Character|GetCharacterMovement _ascreature_character)))))))
            (:then
              (bind _output_get (LocalVariables|SettmpVector (Math|Vector|MakeVector (Math|Random|RandomFloatinRange (.X (Math|Vector|BreakVector (.Min (Components|StaticMesh|GetLocalBounds (Variables|/Script/Engine.StaticMeshActor|GetStaticMeshComponent _asfloor_blueprint))))) (.X (Math|Vector|BreakVector (.Max (Components|StaticMesh|GetLocalBounds (Variables|/Script/Engine.StaticMeshActor|GetStaticMeshComponent _asfloor_blueprint)))))) (Math|Random|RandomFloatinRange (.Y (Math|Vector|BreakVector (.Min (Components|StaticMesh|GetLocalBounds (Variables|/Script/Engine.StaticMeshActor|GetStaticMeshComponent _asfloor_blueprint))))) (.Y (Math|Vector|BreakVector (.Max (Components|StaticMesh|GetLocalBounds (Variables|/Script/Engine.StaticMeshActor|GetStaticMeshComponent _asfloor_blueprint)))))) (LocalVariables|GetSaveZ))))
              (return _output_get))
            (:CastFailed
              (return ""))))
        (:CastFailed
          (return ""))))
    (:CastFailed
      (return ""))))