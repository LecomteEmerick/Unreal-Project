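; Creature_AI_CON is an AI controller that starts and drives creature behavior through a behavior tree.
; On possess, it loads the Creature_AI_BBD blackboard and seeds TargetLocation with the pawn's current location and AIState with the first AiState enum value.
; It then runs Creature_AI_BT, leaving all further logic to the tree, as Tick and the construction script are empty.
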(event `self.OnPossess`
  (params (PossessedPawn :type "Pawn Object Reference"))
  (`self.UseBlackboard` "/Game/Blueprints/Creature_AI_Folder/Creature_AI_BBD.Creature_AI_BBD")
  (`BlackboardComponent.SetValueAsVector` (`AIBlueprintHelperLibrary.GetBlackboard` self) (`self.TargetLocation`) (`self.K2_GetActorLocation` (`self.K2_GetPawn`)))
  (`BlackboardComponent.SetValueAsEnum` (`AIBlueprintHelperLibrary.GetBlackboard` self) (`self.AIState`) (enumliteral `/Game/Blueprints/Creature_AI_Folder/AiState` "NewEnumerator0"))
  (`self.RunBehaviorTree` "/Game/Blueprints/Creature_AI_Folder/Creature_AI_BT.Creature_AI_BT"))

(event `self.ReceiveTick`
  (params (DeltaSeconds :type "Float (single-precision)")))

(fn `UserConstructionScript`)